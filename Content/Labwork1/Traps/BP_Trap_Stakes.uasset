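; Stake trap actor that springs when its pressure plate is overlapped and deals damage over time.
; The plate overlap sets an activation flag, doubles the scale of five stakes and destroys the plate, so it triggers once.
; Any stake overlap sets or clears one shared inside-trap flag without checking the actor.
; Tick calls DamagePlayer, defined outside this graph, with Damage scaled by delta time.
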(event OnComponentBeginOverlap(PressurePlate)
  (params (OverlappedComponent :type Primitive%20Component%20Object%20Reference) (OtherActor :type Actor%20Object%20Reference) (OtherComp :type Primitive%20Component%20Object%20Reference) (OtherBodyIndex :type Integer) (bFromSweep :type Boolean) (SweepResult :type Hit%20Result%20Structure%20%28by%20ref%29))
  (Variables|Default|SetIsPressurePlateActivated true)
  (Transformation|SetRelativeScale3D (Variables|Default|GetStake1) "2.000000,2.000000,2.000000")
  (Transformation|SetRelativeScale3D (Variables|Default|GetStake2) "2.000000,2.000000,2.000000")
  (Transformation|SetRelativeScale3D (Variables|Default|GetStake3) "2.000000,2.000000,2.000000")
  (Transformation|SetRelativeScale3D (Variables|Default|GetStake4) "2.000000,2.000000,2.000000")
  (Transformation|SetRelativeScale3D (Variables|Default|GetStake5) "2.000000,2.000000,2.000000")
  (Components|DestroyComponent (Variables|Default|GetPressurePlate)))

(event OnComponentBeginOverlap(Stake1)
  (params (OverlappedComponent :type Primitive%20Component%20Object%20Reference) (OtherActor :type Actor%20Object%20Reference) (OtherComp :type Primitive%20Component%20Object%20Reference) (OtherBodyIndex :type Integer) (bFromSweep :type Boolean) (SweepResult :type Hit%20Result%20Structure%20%28by%20ref%29))
  (Variables|Default|SetIsPlayerInsideTrap true))

(event OnComponentBeginOverlap(Stake5)
  (params (OverlappedComponent :type Primitive%20Component%20Object%20Reference) (OtherActor :type Actor%20Object%20Reference) (OtherComp :type Primitive%20Component%20Object%20Reference) (OtherBodyIndex :type Integer) (bFromSweep :type Boolean) (SweepResult :type Hit%20Result%20Structure%20%28by%20ref%29))
  (Variables|Default|SetIsPlayerInsideTrap true))

(event OnComponentEndOverlap(Stake5)
  (params (OverlappedComponent :type Primitive%20Component%20Object%20Reference) (OtherActor :type Actor%20Object%20Reference) (OtherComp :type Primitive%20Component%20Object%20Reference) (OtherBodyIndex :type Integer))
  (Variables|Default|SetIsPlayerInsideTrap false))

(event OnComponentEndOverlap(Stake1)
  (params (OverlappedComponent :type Primitive%20Component%20Object%20Reference) (OtherActor :type Actor%20Object%20Reference) (OtherComp :type Primitive%20Component%20Object%20Reference) (OtherBodyIndex :type Integer))
  (Variables|Default|SetIsPlayerInsideTrap false))

(event OnComponentBeginOverlap(Stake2)
  (params (OverlappedComponent :type Primitive%20Component%20Object%20Reference) (OtherActor :type Actor%20Object%20Reference) (OtherComp :type Primitive%20Component%20Object%20Reference) (OtherBodyIndex :type Integer) (bFromSweep :type Boolean) (SweepResult :type Hit%20Result%20Structure%20%28by%20ref%29))
  (Variables|Default|SetIsPlayerInsideTrap true))

(event OnComponentEndOverlap(Stake2)
  (params (OverlappedComponent :type Primitive%20Component%20Object%20Reference) (OtherActor :type Actor%20Object%20Reference) (OtherComp :type Primitive%20Component%20Object%20Reference) (OtherBodyIndex :type Integer))
  (Variables|Default|SetIsPlayerInsideTrap false))

(event OnComponentBeginOverlap(Stake3)
  (params (OverlappedComponent :type Primitive%20Component%20Object%20Reference) (OtherActor :type Actor%20Object%20Reference) (OtherComp :type Primitive%20Component%20Object%20Reference) (OtherBodyIndex :type Integer) (bFromSweep :type Boolean) (SweepResult :type Hit%20Result%20Structure%20%28by%20ref%29))
  (Variables|Default|SetIsPlayerInsideTrap true))

(event OnComponentEndOverlap(Stake3)
  (params (OverlappedComponent :type Primitive%20Component%20Object%20Reference) (OtherActor :type Actor%20Object%20Reference) (OtherComp :type Primitive%20Component%20Object%20Reference) (OtherBodyIndex :type Integer))
  (Variables|Default|SetIsPlayerInsideTrap false))

(event OnComponentBeginOverlap(Stake4)
  (params (OverlappedComponent :type Primitive%20Component%20Object%20Reference) (OtherActor :type Actor%20Object%20Reference) (OtherComp :type Primitive%20Component%20Object%20Reference) (OtherBodyIndex :type Integer) (bFromSweep :type Boolean) (SweepResult :type Hit%20Result%20Structure%20%28by%20ref%29))
  (Variables|Default|SetIsPlayerInsideTrap true))

(event OnComponentEndOverlap(Stake4)
  (params (OverlappedComponent :type Primitive%20Component%20Object%20Reference) (OtherActor :type Actor%20Object%20Reference) (OtherComp :type Primitive%20Component%20Object%20Reference) (OtherBodyIndex :type Integer))
  (Variables|Default|SetIsPlayerInsideTrap false))

(event EventBeginPlay
  (|CallParentFunction) ; This node is disabled and will not be called.\nDrag off pins to build functionality.
)

(event Collision|EventActorBeginOverlap
  (params (OtherActor :type Actor%20Object%20Reference))
  (|CallParentFunction OtherActor) ; This node is disabled and will not be called.\nDrag off pins to build functionality.
)

(event EventTick
  (params (DeltaSeconds :type Float%20%28single-precision%29))
  (|CallParentFunction DeltaSeconds)
  (CallFunction|DamagePlayer (* (Variables|Default|GetDamage) DeltaSeconds)))

(fn ConstructionScript
  (|CallParentFunction))