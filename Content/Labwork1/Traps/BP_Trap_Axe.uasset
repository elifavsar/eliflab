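; Swinging axe trap that stays still until a rope is triggered, then damages the player on contact.
; Overlapping any of four ropes activates the axe and destroys all rope components.
; While active, Tick accumulates time to drive a sine-based roll of the axe root, producing a pendulum swing.
; Axe overlaps apply fixed damage without checking the overlapping actor, briefly toggling the player-inside flag around the damage call.
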(event OnComponentBeginOverlap(Rope3)
  (params (OverlappedComponent :type Primitive%20Component%20Object%20Reference) (OtherActor :type Actor%20Object%20Reference) (OtherComp :type Primitive%20Component%20Object%20Reference) (OtherBodyIndex :type Integer) (bFromSweep :type Boolean) (SweepResult :type Hit%20Result%20Structure%20%28by%20ref%29))
  (CallFunction|RopeEvent))

(event OnComponentBeginOverlap(Rope4)
  (params (OverlappedComponent :type Primitive%20Component%20Object%20Reference) (OtherActor :type Actor%20Object%20Reference) (OtherComp :type Primitive%20Component%20Object%20Reference) (OtherBodyIndex :type Integer) (bFromSweep :type Boolean) (SweepResult :type Hit%20Result%20Structure%20%28by%20ref%29))
  (CallFunction|RopeEvent))

(event OnComponentBeginOverlap(Rope2)
  (params (OverlappedComponent :type Primitive%20Component%20Object%20Reference) (OtherActor :type Actor%20Object%20Reference) (OtherComp :type Primitive%20Component%20Object%20Reference) (OtherBodyIndex :type Integer) (bFromSweep :type Boolean) (SweepResult :type Hit%20Result%20Structure%20%28by%20ref%29))
  (CallFunction|RopeEvent))

(event OnComponentBeginOverlap(Rope1)
  (params (OverlappedComponent :type Primitive%20Component%20Object%20Reference) (OtherActor :type Actor%20Object%20Reference) (OtherComp :type Primitive%20Component%20Object%20Reference) (OtherBodyIndex :type Integer) (bFromSweep :type Boolean) (SweepResult :type Hit%20Result%20Structure%20%28by%20ref%29))
  (CallFunction|RopeEvent))

(event OnComponentBeginOverlap(Axe)
  (params (OverlappedComponent :type Primitive%20Component%20Object%20Reference) (OtherActor :type Actor%20Object%20Reference) (OtherComp :type Primitive%20Component%20Object%20Reference) (OtherBodyIndex :type Integer) (bFromSweep :type Boolean) (SweepResult :type Hit%20Result%20Structure%20%28by%20ref%29))
  (Variables|Default|SetIsPlayerInsideTrap true)
  (CallFunction|DamagePlayer 34.0)
  (Variables|Default|SetIsPlayerInsideTrap false))

(event EventBeginPlay
  (|CallParentFunction) ; This node is disabled and will not be called.\nDrag off pins to build functionality.
)

(event Collision|EventActorBeginOverlap
  (params (OtherActor :type Actor%20Object%20Reference))
  (|CallParentFunction OtherActor) ; This node is disabled and will not be called.\nDrag off pins to build functionality.
)

(event EventTick
  (params (DeltaSeconds :type Float%20%28single-precision%29))
  (|CallParentFunction DeltaSeconds)
  (if (Variables|Default|GetIsAxeActivated)
    (Variables|Default|SetTime (+ DeltaSeconds (Variables|Default|GetTime)))
    (CallFunction|AxeMovement)))

(fn ConstructionScript
  (|CallParentFunction))

(fn AxeMovement
  (bind _axeroot (Variables|Default|GetAxeRoot))
  (bind _relativerotation (Variables|/Script/Engine.SceneComponent|GetRelativeRotation _axeroot))
  (bind _output_get (Variables|Default|SetSinVal (* (Math|Trig|Sin(Degrees) (* (Variables|Default|GetTime) 3.6e+02)) 45.0)))
  (Transformation|SetRelativeRotation _axeroot (Math|Rotator|MakeRotator (+ _output_get 1.8e+02) (.pitch _relativerotation) (.yaw _relativerotation)) false false))

(fn RopeEvent
  (Variables|Default|SetIsAxeActivated true)
  (Components|DestroyComponent (Variables|Default|GetRope4))
  (Components|DestroyComponent (Variables|Default|GetRope3))
  (Components|DestroyComponent (Variables|Default|GetRope2))
  (Components|DestroyComponent (Variables|Default|GetRope1)))