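; BP_Door is a locked door that slides open when interacted with, provided the player has the matching key.
; It caches Gamemode1 on BeginPlay and opens only if that game mode's Keys value equals the door's KeyNumber, otherwise printing a wrong-key message.
; A timeline lerps the Door component's relative location between start and end positions.
; The construction script applies a configurable material to the door.
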(event EventBeginPlay
  (bind _asgamemode_1 (Utilities|Casting|CastToGamemode1 (Game|GetGameMode)))
  (Variables|Default|SetAs%20Gamemode%201 _asgamemode_1))

(event EventInteract
  (if (== (Variables|/Game/Labwork1/Gamemode1.Gamemode1_C|GetKeys (Variables|Default|GetAs%20Gamemode%201)) (Variables|Default|GetKeyNumber))
    (bind _newtrack_0 (Timeline|MoveTemplate Play)
      (:Update
        (Transformation|SetRelativeLocation (Variables|Default|GetDoor) (Math|Vector|Lerp(Vector) (Variables|Default|GetStartLocation) (Variables|Default|GetEndLocaion) _newtrack_0) false false)))
    (else
      (Development|PrintText "You don't have the correct key"))))

(fn ConstructionScript
  (Rendering|Material|SetMaterial (Variables|Default|GetDoor) 0 (Variables|Default|GetMaterial)))