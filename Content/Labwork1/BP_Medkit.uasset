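; BP_Medkit is an interactable pickup that heals the player and then removes itself from the level.
; On Interact, it casts the player pawn to BP_ThirdPersonCharacter_Copy, calls GainHP with its HealthAmount and destroys the actor.
; The construction script applies configurable StaticMesh and Material variables to its Sphere component.
; BeginPlay caches a Gamemode1 reference, which the rest of the graph does not use.
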(event EventBeginPlay
  (bind _asgamemode_1 (Utilities|Casting|CastToGamemode1 (Game|GetGameMode)))
  (Variables|Default|SetAs%20Gamemode%201 _asgamemode_1))

(event Collision|EventActorBeginOverlap
  (params (OtherActor :type Actor%20Object%20Reference)))

(event EventTick
  (params (DeltaSeconds :type Float%20%28single-precision%29)))

(event EventInteract
  (bind _asbp_third_person_character_copy (Utilities|Casting|CastToBP_ThirdPersonCharacter_Copy (Game|Player|GetPlayerPawn 0)))
  (Default|GainHP _asbp_third_person_character_copy (Variables|Default|GetHealthAmount))
  (Actor|DestroyActor))

(fn ConstructionScript
  (bind _sphere (Variables|Default|GetSphere))
  (Components|StaticMesh|SetStaticMesh _sphere (Variables|Default|GetStaticMesh))
  (Rendering|Material|SetMaterial _sphere 0 (Variables|Default|GetMaterial)))