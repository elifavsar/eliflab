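; BP_MazeCell is a modular maze cell actor that builds its floor, optional walls and optional ceiling in the Construction Script.
; GridSize sets the cell footprint and a proportional thickness, while WallHeight sets the vertical size.
; Per-side booleans add static mesh components, scaled through the SizeToCubeScale helper.
; A ceiling with positive LightIntensity also gets a centred point light just below it, using LightColour.
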(event EventBeginPlay)

(event Collision|EventActorBeginOverlap
  (params (OtherActor :type Actor%20Object%20Reference)))

(event EventTick
  (params (DeltaSeconds :type Float%20%28single-precision%29)))

(fn ConstructionScript
  (bind _gridsize (Variables|Default|GetGridSize))
  (LocalVariables|SetWallLenght _gridsize)
  (LocalVariables|SetWallThickness (* _gridsize 0.1))
  (Transformation|SetRelativeScale3D (Variables|Default|GetFloor) (Utilities|SizetoCubeScale (Math|Vector|MakeVector (LocalVariables|GetWallLenght) (LocalVariables|GetWallLenght) (LocalVariables|GetWallThickness))))
  (if (Variables|Default|GetWestWall)
    (AddComponent|AddStaticMeshComponent false (Math|Transform|MakeTransform "0, 0, 0" "0, 0, 0" (Utilities|SizetoCubeScale (Math|Vector|MakeVector (LocalVariables|GetWallLenght) (LocalVariables|GetWallThickness) (Variables|Default|GetWallHeight))))))
  (if (Variables|Default|GetSouthWall)
    (AddComponent|AddStaticMeshComponent false (Math|Transform|MakeTransform "0, 0, 0" "0, 0, 0" (Utilities|SizetoCubeScale (Math|Vector|MakeVector (LocalVariables|GetWallThickness) (LocalVariables|GetWallLenght) (Variables|Default|GetWallHeight))))))
  (if (Variables|Default|GetNorthWall)
    (AddComponent|AddStaticMeshComponent false (Math|Transform|MakeTransform (Math|Vector|MakeVector (- (LocalVariables|GetWallLenght) (LocalVariables|GetWallThickness)) 0.0 0.0) "0, 0, 0" (Utilities|SizetoCubeScale (Math|Vector|MakeVector (LocalVariables|GetWallThickness) (LocalVariables|GetWallLenght) (Variables|Default|GetWallHeight))))))
  (if (Variables|Default|GetEastWall)
    (AddComponent|AddStaticMeshComponent false (Math|Transform|MakeTransform (Math|Vector|MakeVector 0.0 (- (LocalVariables|GetWallLenght) (LocalVariables|GetWallThickness)) 0.0) "0, 0, 0" (Utilities|SizetoCubeScale (Math|Vector|MakeVector (LocalVariables|GetWallLenght) (LocalVariables|GetWallThickness) (Variables|Default|GetWallHeight))))))
  (if (Variables|Default|GetCeiling)
    (AddComponent|AddStaticMeshComponent false (Math|Transform|MakeTransform (Math|Vector|MakeVector 0.0 0.0 (Variables|Default|GetWallHeight)) "0, 0, 0" (Utilities|SizetoCubeScale (Math|Vector|MakeVector (LocalVariables|GetWallLenght) (LocalVariables|GetWallLenght) (LocalVariables|GetWallThickness)))))
    (if (> (Variables|Default|GetLightIntensity) 0.0)
      (bind _returnvalue (AddComponent|AddPointLightComponent false (Math|Transform|MakeTransform (Math|Vector|MakeVector (* (LocalVariables|GetWallLenght) 0.5) (* (LocalVariables|GetWallLenght) 0.5) (* (Variables|Default|GetWallHeight) 0.9)) "0, 0, 0" "1.000000,1.000000,1.000000")))
      (bind _output_get (Variables|Default|SetPointLight _returnvalue))
      (Rendering|Components|Light|SetLightColor _output_get (Variables|Default|GetLightColour) true)
      (Rendering|Components|Light|SetIntensity _output_get (Variables|Default|GetLightIntensity)))))